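; BP_Ball is a physics-driven ball that launches itself along negative X and replaces itself when it goes out of bounds.
; BeginPlay applies a one-time impulse to its Sphere component.
; Each Tick checks the sphere's world X against limits on both sides; crossing either one makes the BP_BallSpawner, looked up by class, spawn a new ball, then destroys this actor.
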(event `self.ReceiveBeginPlay`
  (`PrimitiveComponent.AddImpulse` (`self.Sphere`) (-2500.0 0.0 0.0) "None" false))

(event `self.ReceiveTick`
  (params (DeltaSeconds :type "Float (single-precision)"))
  (bind _returnvalue_x (`KismetMathLibrary.BreakVector` (`SceneComponent.K2_GetComponentLocation` (`self.Sphere`))))
  (if (<= _returnvalue_x -1000.0)
    (bind _returnvalue (`GameplayStatics.GetActorOfClass` "/Game/BP_BallSpawner.BP_BallSpawner_C" :!label _label))
    (`/Game/BP_BallSpawner.SpawnBall` _returnvalue)
    (`self.K2_DestroyActor`)
    (elif (>= _returnvalue_x 1000.0)
      (goto _label))))

(fn `UserConstructionScript`)