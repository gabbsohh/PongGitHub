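; BP_EnemyPaddle is the computer-controlled opponent paddle that follows the ball vertically, apparently for a Pong-style game.
; Each Tick it looks up the BP_Ball actor and, if one exists, calls MoveComponentTo on its Cube.
; The target relative location keeps X fixed and takes Z from the ball's world location, with MoveTime setting the move duration.
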(event `self.ReceiveTick`
  (params (DeltaSeconds :type "Float (single-precision)"))
  (`parent.ReceiveTick` DeltaSeconds)
  ;[1 1 1] checks for ball
  (bind _returnvalue (`GameplayStatics.GetActorOfClass` "/Game/BP_Ball.BP_Ball_C"))
  (if (!= _returnvalue null)
    (bind (_returnvalue_x _returnvalue_y _returnvalue_z) (`KismetMathLibrary.BreakVector` (`self.K2_GetActorLocation` _returnvalue)))
    (`KismetSystemLibrary.MoveComponentTo` (`self.Cube`) (`KismetMathLibrary.MakeVector` 750.0 0.0 _returnvalue_z) (struct) false false (`self.moveTime`))))

(fn `UserConstructionScript`
  (`parent.UserConstructionScript`))